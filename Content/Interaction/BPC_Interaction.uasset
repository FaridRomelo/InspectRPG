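; Actor component that lets its owner detect, interact with and inspect world objects implementing BPI_Interaction.
; A looping 0.2-second timer runs a forward sphere trace (despite the CapsuleTrace name), caching TargetActor and showing its look-at text in WB_InteractMessage.
; Interact and Inspect inputs call the target through interface messages.
; Inspect also removes the prompt widget from its parent, with no re-add here.
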(event Custom|BeginInteraction
  ;[1 1 1] Запуск капусулы через 0,2 секунды
  (Utilities|Time|SetTimerbyEvent (delegate Custom|UpdateInteraction) 0.2 true))

(event Custom|UpdateInteraction
  ;[1 1 1] Запуск капусулы через 0,2 секунды
  (CallFunction|CapsuleTrace))

(event Input|EnhancedActionEvents|EnhancedInputActionAI_Interact
  (params (ActionValue :type Boolean) (ElapsedSeconds :type Float%20%28double-precision%29) (TriggeredSeconds :type Float%20%28double-precision%29) (InputAction :type Input%20Action%20Object%20Reference :default "/Game/ThirdPerson/Input/Actions/AI_Interact.AI_Interact"))
  (:Started
    (bind _targetactor (Variables|Default|GetTargetActor)
      (:then
        (Class|BPIInteraction|Interactwith(Message) _targetactor (CallFunction|GetMyPlayer))
        (Development|PrintString "Interacting"))
      (:else))))

(event Input|EnhancedActionEvents|EnhancedInputActionAI_Inspect
  (params (ActionValue :type Boolean) (ElapsedSeconds :type Float%20%28double-precision%29) (TriggeredSeconds :type Float%20%28double-precision%29) (InputAction :type Input%20Action%20Object%20Reference :default "/Game/ThirdPerson/Input/Actions/AI_Inspect.AI_Inspect"))
  ;[1 1 1] Проверка отключения виджета когда подходишь к объекту
  (:Started
    (bind _targetactor (Variables|Default|GetTargetActor)
      (:then
        (Class|BPIInteraction|Inspect(Message) _targetactor)
        (Development|PrintString "Inspecting" true true "(R=1.000000,G=0.144617,B=0.000000,A=1.000000)")
        (Widget|RemovefromParent (Variables|Default|GetWB_InteractMessage)))
      (:else))))

(event EventBeginPlay
  (CallFunction|CreateInteractMessage)
  (CallFunction|BeginInteraction))

(fn CreateInteractMessage
  (bind _returnvalue (Game|ConstructObjectfromClass "/Game/Interaction/UI/WB_InteractMessage.WB_InteractMessage_C"))
  (bind _output_get (Variables|Default|SetWB_InteractMessage _returnvalue))
  (UserInterface|Viewport|AddtoViewport _output_get 0))

(fn CapsuleTrace
  (bind _returnvalue (Components|GetOwner))
  (bind _returnvalue_2 (Transformation|GetActorLocation _returnvalue))
  ;[1 1 1] Трасировка взаимодействия с объектом капсула
  (bind (_outhit _returnvalue_3) (Collision|SphereTraceByChannel _returnvalue_2 (+ _returnvalue_2 (* (Transformation|GetActorForwardVector _returnvalue) 1.5e+02)) 8e+01 "TraceTypeQuery3" false 0 "None"))
  (if _returnvalue_3
    (if (Utilities|DoesObjectImplementInterface (.HitActor (Collision|BreakHitResult _outhit)) "/Game/Interaction/BPI_Interaction.BPI_Interaction_C")
      (bind _output_get (Variables|Default|SetTargetActor (.HitActor (Collision|BreakHitResult _outhit))))
      (bind _message (Class|BPIInteraction|Lookat(Message) _output_get))
      (Default|SetMessage (Variables|Default|GetWB_InteractMessage) _message)
      (else
        (Variables|Default|SetTargetActor 0)
        (Default|SetMessage (Variables|Default|GetWB_InteractMessage))))
    (else
      (Variables|Default|SetTargetActor 0)
      (Default|SetMessage (Variables|Default|GetWB_InteractMessage)))))